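; BP_Fence is a fence actor that swings open once enough flies have been eaten.
; The Eatflies event increments a collected-fly counter and, on reaching the maximum, fires Openfence a single time through a DoOnce.
; Openfence plays the Opening timeline, whose curve lerps the fence's relative yaw to rotate it open.
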(event `Openfence`
  ; Animation pour l'ouverture de la cloture
  (bind (_direction _anim) (`Timeline|Opening`)
    (:`Update`
      (`SceneComponent.K2_SetRelativeRotation` (`self.Fence`) (`KismetMathLibrary.MakeRotator` 0.0 0.0 (`KismetMathLibrary.Lerp` 0.0 40.0 _anim)) false false))))

(event `Eat flies`
  ; Calcul pour ouvrir une cloture
  (`/Engine/EditorBlueprintResources/StandardMacros.IncrementInt` (`self.Mouche collecter`)
    (:`  `
      (if (>= (`self.Mouche collecter`) (`self.Mouche maximum`))
        (`/Engine/EditorBlueprintResources/StandardMacros.DoOnce` false
          (:`Completed`
            (`self.Openfence`)))))))

(fn `UserConstructionScript`)