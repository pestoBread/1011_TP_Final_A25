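; BP_PuzzleGate is a puzzle gate that reacts once enough items have been collected.
; CollectItem increments a counter and, when it reaches MaxItems, fires RaisePlatform once through a DoOnce.
; RaisePlatform plays the ActionRaise timeline, whose Raising track lerps the Platform's relative yaw from 0 to 30 degrees, so the platform rotates rather than moving upward despite the name.
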(event `RaisePlatform`
  (bind (_direction _raising) (`Timeline|ActionRaise`)
    (:`Update`
      (`SceneComponent.K2_SetRelativeRotation` (`self.Platform`) (`KismetMathLibrary.MakeRotator` 0.0 0.0 (`KismetMathLibrary.Lerp` 0.0 30.0 _raising)) false false))))

(event `Collect Item`
  (`/Engine/EditorBlueprintResources/StandardMacros.IncrementInt` (`self.CurrentItems`)
    (:`  `
      (if (>= (`self.CurrentItems`) (`self.MaxItems`))
        (`/Engine/EditorBlueprintResources/StandardMacros.DoOnce` false
          (:`Completed`
            (`self.RaisePlatform`)))))))

(fn `UserConstructionScript`)