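; AC_HealthSystem is a health component that tracks current health against a maximum and reports damage and death.
; Current health starts at the maximum on BeginPlay, and DecreaseHealth removes one point per call.
; A non-lethal hit broadcasts OnHealthChange with current and maximum health and prints the new value.
; A lethal hit broadcasts only OnDeath, leaving the stored health unchanged.
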(event `self.ReceiveBeginPlay`
  (set `self.CurrentHealth` (`self.MaxHealth`)))

(fn `DecreaseHealth`
  (bind _returnvalue (- (`self.CurrentHealth`) 1))
  (if (<= _returnvalue 0)
    (`self.OnDeath`)
    (else
      (bind _output_get (set `self.CurrentHealth` _returnvalue))
      (`self.OnHealthChange` _output_get (`self.MaxHealth`))
      (`KismetSystemLibrary.PrintText` (`KismetTextLibrary.Conv_IntToText` _output_get)))))