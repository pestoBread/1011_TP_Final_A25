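; Actor component that tracks how many BP_PuzzleItem actors remain to be collected and shows that number on screen.
; On BeginPlay it creates a WBP_FlyCounter widget, adds it to the viewport and seeds the count from all puzzle items in the level.
; DecreaseCounter lowers the count, updates the widget, broadcasts OnCountUpdate, and fires OnZeroCount once the count reaches zero or below.
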(event `self.ReceiveBeginPlay`
  (`|ExecutionSequence`
    (:`then_0`
      (bind _returnvalue (`|CreateWidget` "/Game/_pestoBread/WBP_FlyCounter.WBP_FlyCounter_C" (`GameplayStatics.GetPlayerController` 0)))
      (bind _output_get (set `self.ItemCounterUI` _returnvalue))
      (`UserWidget.AddToViewport` _output_get 0))
    (:`then_1`
      (bind _outactors (`GameplayStatics.GetAllActorsOfClass` "/Game/_walbio/BP_PuzzleItem.BP_PuzzleItem_C"))
      (bind _output_get_2 (set `self.ItemCount` (`KismetArrayLibrary.Array_Length` _outactors)))
      (`self.OnCountUpdate` _output_get_2)
      (`/Game/_pestoBread/WBP_FlyCounter.SetCounterNum` (`self.ItemCounterUI`) _output_get_2))))

(fn `DecreaseCounter`
  (bind _result (`/Engine/EditorBlueprintResources/StandardMacros.DecrementInt` (`self.ItemCount`))
    (:`  `
      (bind _output_get (set `self.ItemCount` _result))
      (`self.OnCountUpdate` _output_get)
      (`/Game/_pestoBread/WBP_FlyCounter.SetCounterNum` (`self.ItemCounterUI`) _output_get)
      (if (<= _output_get 0)
        (`self.OnZeroCount`)))))